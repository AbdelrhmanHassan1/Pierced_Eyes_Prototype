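; BP_GasPuzzle is a gas puzzle actor that places toxic gas effects in the level.
; Its construction script loops over fixed indices, adding a Niagara component at each world location and rotation read from the GasTransform and GasWorldRotation arrays.
; Each component uses NS_ToxicGas with auto-activation off.
; The event graph holds only empty stub events, so this file contains no activation or puzzle logic.
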(event `self.ReceiveTick`
  (params (DeltaSeconds :type "Float (single-precision)")))

(fn `UserConstructionScript`
  (for _index (range 4)
    (set `self.World Transform Location` (`|GetArrayItem` (`self.Gas Transform`) _index))
    (set `self.World Rotaion` (`|GetArrayItem` (`self.Gas World Rotation`) _index))
    (bind _returnvalue (`AddComponent|NODE_AddNiagaraComponent-0`))
    (`SceneComponent.K2_SetWorldLocationAndRotation` _returnvalue (`self.World Transform Location`) (`self.World Rotaion`) false false)
    (`NiagaraComponent.SetAsset` _returnvalue "/Game/AdvancedLocomotionV4_1/Blueprints/VFX_Blueprints/Materials/NS_ToxicGas.NS_ToxicGas" true)
    (`ActorComponent.SetAutoActivate` _returnvalue false)))