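; Fake pressure plate that sets off a referenced BP_GasPuzzle when stepped on by a Locomotion actor.
; Trigger overlap plays a shutter sound, sets IsActive and runs the PlatePressure timeline to lower the plate.
; Leaving waits one second, then plays a second sound, clears IsActive and reverses the timeline.
; ActivateGasPuzzle sits on the timeline update, so it fires repeatedly during both press and release.
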(event `self.Trigger.OnComponentBeginOverlap`
  (params (OverlappedComponent :type "PrimitiveComponent Object Reference") (OtherActor :type "Actor Object Reference") (OtherComp :type "PrimitiveComponent Object Reference") (OtherBodyIndex :type Integer) (bFromSweep :type Boolean) (SweepResult :type "HitResult Structure (by ref)"))
  ;[1 1 1] Plate Activate Logic
  (cast `/Game/AdvancedLocomotionV4_1/Blueprints/CharacterLogic/Locomotion` OtherActor)
  (`GameplayStatics.PlaySoundAtLocation` "/Engine/VREditor/Sounds/UI/Camera_Shutter.Camera_Shutter" (`self.K2_GetActorLocation`) (struct) 1.0 1.0 0.0 null null null null)
  (set `self.isActive` true)
  (if true
    (bind (_direction _highet) (`Timeline|Plate Pressure` :!label _label)
      (:`Update`
        (`SceneComponent.K2_SetRelativeLocation` (`self.Plate`) (`KismetMathLibrary.MakeVector` 0.0 0.0 (`KismetMathLibrary.Lerp` 1.5 -5.0 _highet)) false false)
        (bind _asbp_gas_puzzle (cast `/Game/HorrorEngine/Blueprints/UsableAssets/PortalAndTriggers/BP_GasPuzzle` (`self.Gas Puzzle`)))
        (`/Game/HorrorEngine/Blueprints/UsableAssets/PortalAndTriggers/BP_GasPuzzle.Activate Gas Puzzle` _asbp_gas_puzzle)))
    (else
      (goto _label))))

(event `self.Trigger.OnComponentEndOverlap`
  (params (OverlappedComponent :type "PrimitiveComponent Object Reference") (OtherActor :type "Actor Object Reference") (OtherComp :type "PrimitiveComponent Object Reference") (OtherBodyIndex :type Integer))
  (`KismetSystemLibrary.Delay` 1.0)
  ;[1 1 1] De Activate
  (cast `/Game/AdvancedLocomotionV4_1/Blueprints/CharacterLogic/Locomotion` OtherActor)
  (`GameplayStatics.PlaySoundAtLocation` "/Game/HorrorEngine/Audio/Elecronic/CameraZoomIn.CameraZoomIn" (`self.K2_GetActorLocation`) (struct) 1.0 1.0 0.0 null null null null)
  (set `self.isActive` false)
  (goto _label :!via `Reverse`))

(fn `UserConstructionScript`)