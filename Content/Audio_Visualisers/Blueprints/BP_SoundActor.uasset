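; BP_SoundActor is an audio visualiser actor with a cube that reacts to its audio component, which Tick restarts through a three-second Delay.
; Each play state change spawns the NS_Sound_Wave Niagara system at the cube and nudges the cube along world Y.
; SetSize scales cube height from cooked envelope data above a minimum threshold, but is not called within this Blueprint.
; Audio finishing flattens the cube.
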(event `OnAudioFinished_Event`
  (`SceneComponent.SetRelativeScale3D` (`self.Cube`) (1.0 1.0 0.1)))

(event `self.ReceiveTick`
  (params (DeltaSeconds :type "Float (single-precision)"))
  (`KismetSystemLibrary.Delay` 3.0)
  (`AudioComponent.Play` (`self.Audio`) 0.0))

(event `self.ReceiveBeginPlay`
  (add `AudioComponent.OnAudioPlayStateChanged` (`self.Audio`) (delegate `OnAudioPlayStateChanged_Event`))
  (add `AudioComponent.OnAudioFinished` (`self.Audio`) (delegate `OnAudioFinished_Event`)))

(event `OnAudioPlayStateChanged_Event`
  (params (PlayState :type "EAudioComponentPlayState Enum" :default "Playing"))
  (bind (_returnvalue_x _returnvalue_y _returnvalue_z) (`KismetMathLibrary.BreakVector` (`SceneComponent.K2_GetComponentLocation` (`self.Cube`))))
  (`|ExecutionSequence`
    (:`then_0`
      (`NiagaraFunctionLibrary.SpawnSystemAtLocation` "/Game/Audio_Visualisers/Niagra/NS_Sound_Wave.NS_Sound_Wave" (`SceneComponent.K2_GetComponentLocation` (`self.Cube`))))
    (:`then_1`
      (`SceneComponent.K2_SetWorldLocation` (`self.Cube`) (`KismetMathLibrary.MakeVector` _returnvalue_x (+ _returnvalue_y 2.0) _returnvalue_z) false false))))

(fn `SetSize`
  (bind _outenvelopedata (`AudioComponent.GetCookedEnvelopeData` (`self.Audio`)))
  (bind _returnvalue (* _outenvelopedata 20.0))
  (if (>= _returnvalue 0.1)
    (`SceneComponent.SetRelativeScale3D` (`self.Cube`) (`KismetMathLibrary.MakeVector` 1.0 1.0 _returnvalue))))

(fn `UserConstructionScript`)